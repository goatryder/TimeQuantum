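; AmmoBox_BP is an ammo pickup that gradually refills the player's ammo while MainPlayerCharacter_BP overlaps it.
; Tick accumulates a timer during overlap and, past a threshold, moves one round from the box to the player if below max, playing audio and updating a text counter.
; When the box empties, a timeline shrinks it from its initial scale to zero, then destroys it.
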(event Custom|OnDestroy
  ;[1 1 1] Shrink And Destroy Cube
  (bind _alpha (Timeline|BoxShrinkTemplate Play)
    (:Update
      (Transformation|SetActorScale3D (Math|Vector|Lerp(Vector) (Variables|Default|GetCurrentScale) "0, 0, 0" _alpha)))
    (:Finished
      (Actor|DestroyActor))))

(event EventBeginPlay
  ;[1 1 1] Display Initial Ammo
  (Rendering|Components|TextRender|SetText (Variables|Default|GetTextAmmoCount) (Utilities|Text|ToText(Integer) (Variables|Default|GetAmmoLeft)))
  ;[1 1 1] Set Initial Scale
  (Variables|Default|SetCurrentScale (Transformation|GetActorScale3D)))

(event Collision|EventActorBeginOverlap
  (params (OtherActor :type Actor%20Object%20Reference))
  (bind _asmain_player_character_bp (Utilities|Casting|CastToMainPlayerCharacter_BP OtherActor))
  (Variables|Default|SetPlayerREF _asmain_player_character_bp)
  (Variables|Default|SetCanFillAmmo true))

(event EventTick
  (params (DeltaSeconds :type Float%20%28single-precision%29))
  (bind _playerref (Variables|Default|GetPlayerREF))
  (if (Variables|Default|GetCanFillAmmo)
    (bind _output_get (Variables|Default|SetFillAmmoTimer (+ (Variables|Default|GetFillAmmoTimer) DeltaSeconds)))
    (if (>= _output_get (Variables|Default|GetFillAmmoTreshold))
      (if (< (Variables|/Game/Blueprints/Character_BP/MainPlayerCharacter_BP.MainPlayerCharacter_BP_C|GetCurrentAmmo _playerref) (Variables|/Game/Blueprints/Character_BP/MainPlayerCharacter_BP.MainPlayerCharacter_BP_C|GetMaxAmmo _playerref))
        (Math|Integer|IncrementInt (Variables|/Game/Blueprints/Character_BP/MainPlayerCharacter_BP.MainPlayerCharacter_BP_C|GetCurrentAmmo (Variables|Default|GetPlayerREF))
          (:%20%20
            (bind _result (Math|Integer|DecrementInt (Variables|Default|GetAmmoLeft))
              (:%20%20
                (Rendering|Components|TextRender|SetText (Variables|Default|GetTextAmmoCount) (Utilities|Text|ToText(Integer) _result))
                (Variables|Default|SetFillAmmoTimer 0.0)
                (Audio|Components|Audio|Play (Variables|Default|GetAudio) 0.0)
                (if (== (Variables|Default|GetAmmoLeft) 0)
                  (if (Variables|Default|GetCanDestroy)
                    (Variables|Default|SetCanDestroy false)
                    (CallFunction|OnDestroy)))))))))))

(event Collision|EventActorEndOverlap
  (params (OtherActor :type Actor%20Object%20Reference))
  (Utilities|Casting|CastToMainPlayerCharacter_BP OtherActor)
  (Variables|Default|SetCanFillAmmo false)
  (Variables|Default|SetFillAmmoTimer 0.0))

(fn ConstructionScript)