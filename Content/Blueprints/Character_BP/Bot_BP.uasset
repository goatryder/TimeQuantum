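; Enemy bot that turns toward the player and shoots, registering itself and its death with Game_Mode_Controller.
; A looping timer line-traces from the head socket to the player's camera, setting target and yaw when visible within range.
; Tick lerps toward that yaw and fires the socket-attached gun at a set rate once a dot-product cone check passes, using a reversed forward axis.
; Death ragdolls the mesh and gun.
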(event Custom|Death
  (if (Variables|Default|GetIsAlive)
    (Variables|Default|SetIsAlive false)
    (Physics|SetSimulatePhysics (Variables|Default|GetMesh) true)
    (Physics|SetSimulatePhysics (Variables|/Game/Blueprints/Weapons_BP/Gun_Bot_BP.Gun_Bot_BP_C|GetGunMesh (Variables|Default|GetGun)) true)
    (bind _asgame_mode_controller (Utilities|Casting|CastToGame_Mode_Controller (Game|GetGameMode)))
    (Default|BotKilled _asgame_mode_controller)))

(event EventBeginPlay
  ;[1 1 1] attach gun
  (CallFunction|SpawnandAttachGun)
  ;[1 1 1] RegisterBot
  (bind _asgame_mode_controller (Utilities|Casting|CastToGame_Mode_Controller (Game|GetGameMode)))
  (Default|RegisterBot _asgame_mode_controller)
  ;[1 1 1] Get Reference To Player And Angle To Rotate Towards The Player
  (Utilities|Time|SetTimerbyFunctionName self "CheckForPlayer" 0.1 true))

(event EventTick
  (params (DeltaSeconds :type Float%20%28single-precision%29))
  (if (Variables|Default|GetIsAlive)
    ;[1 1 1] Rotate To Player
    (if (CallFunction|CheckShouldRotate)
      (Utilities|IsValid (Variables|Default|GetTargetActor)
        (:Is%20Valid
          (Variables|Default|SetLockTimer true)
          (CallFunction|RotatetoPlayer DeltaSeconds)
          (Variables|Default|SetLockTimer false)
          (bind _output_get (Variables|Default|SetCanSeePlayer (CallFunction|PlayerinViewRange)))
          ;[1 1 1] If Can See Player
          (if _output_get
            ;[1 1 1] Shoot Player
            (bind _output_get_2 (Variables|Default|SetCanFire (+ (Variables|Default|GetCanFire) (* (Variables|Default|GetFireRate) DeltaSeconds))))
            (if (> _output_get_2 (Variables|Default|GetFireTreshold))
              (Default|FireBullet (Variables|Default|GetGun))
              (Variables|Default|SetCanFire 0.0)
              (Variables|Default|SetShootEvent true)
              (else
                (Variables|Default|SetShootEvent false)))))
        (:Is%20Not%20Valid
          (Variables|Default|SetLockTimer false :!label _label)
          (Variables|Default|SetCanSeePlayer false)))
      (else
        (goto _label)))
    (else
      (goto _label))))

(fn ConstructionScript)

(fn SpawnandAttachGun
  (bind _returnvalue (Game|SpawnActorfromClass "/Game/Blueprints/Weapons_BP/Gun_Bot_BP.Gun_Bot_BP_C" (Transformation|GetSocketTransform (Variables|Default|GetMesh) "b_Gun" "RTS_World") "Undefined" 0 0))
  (bind _output_get (Variables|Default|SetGun _returnvalue))
  (Transformation|AttachComponentToComponent _output_get (Variables|Default|GetMesh) "b_Gun" "KeepWorld" "KeepWorld" "KeepWorld" true))

(fn CheckforPlayer
  (bind _asmain_player_character_bp (Utilities|Casting|CastToMainPlayerCharacter_BP (Game|GetPlayerCharacter 0)))
  (bind _outhit (Collision|LineTraceByChannel (.Location (Math|Transform|BreakTransform (Transformation|GetSocketTransform (Variables|Default|GetMesh) "headSocket" "RTS_World"))) (+ (Transformation|GetActorLocation (Game|GetPlayerCharacter 0)) (Variables|/Script/Engine.SceneComponent|GetRelativeLocation (Variables|/Game/Blueprints/Character_BP/MainPlayerCharacter_BP.MainPlayerCharacter_BP_C|GetFPS_Camera _asmain_player_character_bp))) "TraceTypeQuery2" false 0 "None"))
  (LocalVariables|SetHitActor (.HitActor (Collision|BreakHitResult _outhit)))
  ;[1 1 1] Hit Actor Is Not Null
  (if (|HitActorIsNotNull)
    ;[1 1 1] Hit Actor Is Player Character
    (if (|HitActorIsPlayer)
      ;[1 1 1] Player Character in View Range
      (if (|PlayerinDistanceRange)
        (Variables|Default|SetDesiredRotation (Math|Rotator|FindLookatRotation (Transformation|GetActorLocation (LocalVariables|GetHitActor)) (Transformation|GetActorLocation)))
        (Variables|Default|SetTargetActor (LocalVariables|GetHitActor))
        (else
          (if (not (Variables|Default|GetLockTimer)) :!label _label
            (Variables|Default|SetTargetActor 0))))
      (else
        (goto _label)))))

(fn CheckShouldRotate
  (bind _returnvalue (Transformation|GetActorRotation))
  (bind _desiredrotation (Variables|Default|GetDesiredRotation))
  (bind _yaw (Math|Rotator|BreakRotator _returnvalue))
  (bind _yaw_2 (Math|Rotator|BreakRotator _desiredrotation))
  (return (or (!= _yaw _yaw_2) (== _yaw _yaw_2))))

(fn RotatetoPlayer
  (params (DeltaSeconds :type Float%20%28single-precision%29))
  (Transformation|SetActorRotation (Math|Rotator|Lerp(Rotator) (Transformation|GetActorRotation) (Math|Rotator|MakeRotator 0.0 0.0 (.Yaw (Math|Rotator|BreakRotator (Variables|Default|GetDesiredRotation)))) (* DeltaSeconds (Variables|Default|GetRotateRate)) true)))

(fn PlayerinViewRange
  (return (< (Math|Vector|DotProduct (Math|Vector|Normalize (Math|Rotator|GetRotationXVector (Transformation|GetActorRotation))) (Math|Vector|Normalize (Math|Vector|GetUnitDirection(Vector) (Transformation|GetActorLocation) (Transformation|GetActorLocation (Variables|Default|GetTargetActor))))) -0.85)))